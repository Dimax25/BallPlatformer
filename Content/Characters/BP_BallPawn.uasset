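; BP_BallPawn is a player-controlled ball pawn that moves through physics forces and can jump.
; Move axes scale the camera's forward and right vectors by input and BallSpeed in GetMovementDirection, then apply the result to the mesh as mass-independent force.
; Look axes drive controller pitch and yaw.
; Space adds an upward force only when the mesh's height is at or below FloorLevel, with no collision-based ground check.
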(event EventBeginPlay)

(event Collision|EventActorBeginOverlap
  (params (OtherActor :type Actor%20Object%20Reference)))

(event EventTick
  (params (DeltaSeconds :type Float%20%28single-precision%29)))

(event Input|AxisEvents|InputAxisMoveForwardBackwards
  (params (AxisValue :type Float%20%28single-precision%29))
  (bind _camera (Variables|Default|GetCamera))
  (bind _returnvalue (Math|Vector|GetForwardVector _camera))
  (bind (_staticmesh _resulting_force_vector) (CallFunction|GetMovementDirection _returnvalue AxisValue))
  ;[1 1 1] Basic Player Movement
  (Physics|AddForce _staticmesh _resulting_force_vector "None" true))

(event Input|AxisEvents|InputAxisMoveLeftRight
  (params (AxisValue :type Float%20%28single-precision%29))
  (bind _camera (Variables|Default|GetCamera))
  (bind _returnvalue (Math|Vector|GetRightVector _camera))
  (bind (_staticmesh _resulting_force_vector) (CallFunction|GetMovementDirection _returnvalue AxisValue))
  ;[1 1 1] Basic Player Movement
  (Physics|AddForce _staticmesh _resulting_force_vector "None" true))

(event Input|AxisEvents|InputAxisTurn
  (params (AxisValue :type Float%20%28single-precision%29))
  ;[1 1 1] Basic Camera Movement
  (Pawn|Input|AddControllerYawInput AxisValue))

(event Input|AxisEvents|InputAxisLookUp
  (params (AxisValue :type Float%20%28single-precision%29))
  ;[1 1 1] Basic Camera Movement
  (Pawn|Input|AddControllerPitchInput AxisValue))

(event Input|KeyboardEvents|SpaceBar
  (params (Key :type Key%20Structure :default "None"))
  ;[1 1 1] Basic Player Movement
  (:Pressed
    (if (<= (.Z (Math|Vector|BreakVector (Transformation|GetWorldLocation (Variables|Default|GetStaticMesh)))) (Variables|Default|GetFloor%20Level))
      (Development|PrintString "JUMP" true true "(R=0.325521,G=0.651042,B=0.000000,A=1.000000)")
      (Physics|AddForce (Variables|Default|GetStaticMesh) "0.000000,0.000000,50000.000000" "None" true))))

(fn ConstructionScript)

(fn GetMovementDirection
  (params (Camera%20Direction :type Vector) (Axis%20Input%20Value :type Float%20%28single-precision%29))
  (return (Variables|Default|GetStaticMesh) (* (* Camera%20Direction Axis%20Input%20Value) (Variables|Default|GetBallSpeed))))